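; BrokenEngine is an engine piece actor that flies off at the start of play and snaps onto a PieceSpot it overlaps.
; On BeginPlay, a delayed random-direction impulse launches the static mesh, then timed linear damping changes briefly slow it before freeing it up again.
; On overlap with a PieceSpot, it detaches the mesh, moves the actor to the spot's location and attaches the mesh to the spot's root.
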(event `self.ReceiveBeginPlay`
  (bind _staticmesh (`self.StaticMesh`))
  (`KismetSystemLibrary.Delay` 1.5)
  (`PrimitiveComponent.AddImpulse` (`self.StaticMesh`) (* (`KismetMathLibrary.RandomUnitVector`) 2000) "None" true)
  (`KismetSystemLibrary.Delay` 2.0)
  (`PrimitiveComponent.SetLinearDamping` _staticmesh 5.0)
  (`KismetSystemLibrary.Delay` 3.0)
  (`PrimitiveComponent.SetLinearDamping` _staticmesh 0.01))

(event `self.ReceiveActorBeginOverlap`
  (params (OtherActor :type "Actor Object Reference"))
  (bind _rootcomponent (`Actor.RootComponent` OtherActor))
  (if (== (`GameplayStatics.GetObjectClass` OtherActor) "/Game/Blueprints/PieceSpot.PieceSpot_C")
    (`SceneComponent.K2_DetachFromComponent` (`self.StaticMesh`) "KeepWorld" "KeepWorld" "KeepWorld" true)
    (`self.K2_SetActorLocation` (`SceneComponent.K2_GetComponentLocation` _rootcomponent))
    (`SceneComponent.K2_AttachToComponent` (`self.StaticMesh`) _rootcomponent "None" "KeepWorld" "KeepWorld" "KeepWorld" true)))

(fn `UserConstructionScript`)