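; Button Blueprint with a point light that blinks while the button is enabled and accepts presses only in that state.
; EnableBlink sets the Blink flag, and Tick then drives the light intensity with a time-based sine wave scaled by DefaultIntensity.
; PressButton fires the ButtonPressed dispatcher only while Blink is set.
; Disabling Blink leaves the light at its last intensity.
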(event `self.ReceiveTick`
  (params (DeltaSeconds :type "Float (single-precision)"))
  (if (`self.bBlink`)
    (`self.Blink`)))

(event `Blink`
  (`LightComponent.SetIntensity` (`self.PointLight`) (* (`KismetMathLibrary.Sin` (* (`GameplayStatics.GetTimeSeconds`) 7.0)) (`self.DefaultIntensity`))))

(event `EnableBlink`
  (params (Enable :type Boolean))
  (set `self.bBlink` Enable))

(event `PressButton`
  (if (`self.bBlink`)
    (`self.ButtonPressed`)))

(fn `UserConstructionScript`)