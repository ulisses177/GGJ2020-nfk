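; VR joystick that lets the player steer by grabbing it with the right hand.
; Finds the PlayerShip on BeginPlay and, each tick, snaps the stick mesh to the hand while it is closed and overlapping.
; The mesh's normalized relative offset feeds the VR character's Forward (average of X and Z) and Right (Y) inputs, so only direction counts.
; Otherwise the mesh snaps back to its local origin.
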(event `self.ReceiveBeginPlay`
  (bind _outactors (`GameplayStatics.GetAllActorsOfClass` "/Game/VirtualRealityBP/Blueprints/VrController/RevampPawns/PlayerShip.PlayerShip_C"))
  (set `self.ShipRef` (`|GetArrayItem` _outactors)))

(event `self.ReceiveTick`
  (params (DeltaSeconds :type "Float (single-precision)"))
  (bind _asplayer_ship (cast `/Game/VirtualRealityBP/Blueprints/VrController/RevampPawns/PlayerShip` (`self.ShipRef`)))
  (bind _vrchatacterref (`/Game/VirtualRealityBP/Blueprints/VrController/RevampPawns/PlayerShip.VrChatacterRef` _asplayer_ship))
  (`/Engine/EditorBlueprintResources/StandardMacros.IsValid` _vrchatacterref
    (:`Is Valid`
      (if (and (`/Game/VirtualRealityBP/Blueprints/VrController/VrCharacter.bCloseRightHand` _vrchatacterref) (`PrimitiveComponent.IsOverlappingComponent` (`self.StaticMesh`) (`/Game/VirtualRealityBP/Blueprints/VrController/VrCharacter.RightHandCollision` _vrchatacterref)))
        (`SceneComponent.K2_SetWorldLocation` (`self.StaticMesh`) (`SceneComponent.K2_GetComponentLocation` (`/Game/VirtualRealityBP/Blueprints/VrController/VrCharacter.RHand` _vrchatacterref)) false false)
        (bind _asplayer_ship_2 (cast `/Game/VirtualRealityBP/Blueprints/VrController/RevampPawns/PlayerShip` (`self.ShipRef`)))
        (`|ExecutionSequence`
          (:`then_0`
            (bind _vrchatacterref_2 (`/Game/VirtualRealityBP/Blueprints/VrController/RevampPawns/PlayerShip.VrChatacterRef` _asplayer_ship_2))
            (`/Game/VirtualRealityBP/Blueprints/VrController/VrCharacter.Forward` _vrchatacterref_2 (/ (+ (.x (`KismetMathLibrary.Normal` (`SceneComponent.RelativeLocation` (`self.StaticMesh`)))) (.z (`KismetMathLibrary.Normal` (`SceneComponent.RelativeLocation` (`self.StaticMesh`))))) 2.0)))
          (:`then_1`
            (`/Game/VirtualRealityBP/Blueprints/VrController/VrCharacter.Right` _vrchatacterref_2 (.y (`KismetMathLibrary.Normal` (`SceneComponent.RelativeLocation` (`self.StaticMesh`)))))))
        (else
          (`SceneComponent.K2_SetRelativeLocation` (`self.StaticMesh`) (0.0 0.0 0.0) false false))))))

(fn `UserConstructionScript`)