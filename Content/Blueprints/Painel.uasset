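; Cockpit panel actor with velocity, altitude and damage readouts, simulating ship damage and button-driven repairs.
; BeginPlay caches HUD widgets and the VR character, then binds four child-actor buttons to RepairDamage, which adds health.
; A Tick-driven delay repeats heavy then light hits that flash the panel material, set buttons blinking and conditionally cut health with impact sounds.
; Light hits also refresh the health text and play an engine-failure voice at low health.
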(event `self.ReceiveBeginPlay`
  (`|ExecutionSequence`
    (:`then_0`
      (bind _aswgt_hud (cast `/Game/Blueprints/HUD/WGT_HUD` (`WidgetComponent.GetUserWidgetObject` (`self.Wgt_Velocity`))))
      (set `self.Wgt_Velocity_ref` _aswgt_hud)
      (bind _aswgt_hud_2 (cast `/Game/Blueprints/HUD/WGT_HUD` (`WidgetComponent.GetUserWidgetObject` (`self.Wgt_Damage`))))
      (set `self.Wgt_Damage_ref` _aswgt_hud_2)
      (`self.SetHealth` (`KismetTextLibrary.Conv_DoubleToText` (`self.Health`) "HalfToEven"))
      (`KismetSystemLibrary.Delay` 2.0)
      (`self.HeavyDamage`)
      (`parent.ReceiveBeginPlay`)
      (bind _asvr_character (cast `/Game/VirtualRealityBP/Blueprints/VrController/VrCharacter` (`GameplayStatics.GetPlayerCharacter` 0)))
      (set `self.VrChatacterRef` _asvr_character)
      (`|ExecutionSequence`
        (:`then_0`
          (bind _asbutton (cast `/Game/Blueprints/Button` (`ChildActorComponent.ChildActor` (`self.Button1`))))
          (`KismetArrayLibrary.Array_Add` (`self.Buttons`) _asbutton)
          (bind _asbutton_2 (cast `/Game/Blueprints/Button` (`ChildActorComponent.ChildActor` (`self.Button2`))))
          (`KismetArrayLibrary.Array_Add` (`self.Buttons`) _asbutton_2)
          (bind _asbutton_3 (cast `/Game/Blueprints/Button` (`ChildActorComponent.ChildActor` (`self.Button3`))))
          (`KismetArrayLibrary.Array_Add` (`self.Buttons`) _asbutton_3)
          (bind _asbutton_4 (cast `/Game/Blueprints/Button` (`ChildActorComponent.ChildActor` (`self.Button4`))))
          (`KismetArrayLibrary.Array_Add` (`self.Buttons`) _asbutton_4))
        (:`then_1`
          (for _array_element (`self.Buttons`)
            (add `/Game/Blueprints/Button.ButtonPressed` _array_element (delegate `RepairDamage`))))))
    (:`then_1`
      (`KismetSystemLibrary.Delay` 2.0)
      (`self.HeavyDamage` :!label _label)
      (`KismetSystemLibrary.Delay` 0.2)
      (`self.LightDamage`))))

(event `SetHud`
  (params (Velocity :type Text) (Altitude :type Text) (Damage :type Text))
  (`/Game/Blueprints/HUD/WGT_HUD.SetText` (`self.Wgt_Velocity_ref`) Velocity)
  (`/Game/Blueprints/HUD/WGT_HUD.SetText` (`self.Wgt_Altitude_ref`) Altitude)
  (`/Game/Blueprints/HUD/WGT_HUD.SetText` (`self.Wgt_Damage_ref`) Damage))

(event `self.ReceiveTick`
  (params (DeltaSeconds :type "Float (single-precision)"))
  (`KismetSystemLibrary.Delay` 10.0)
  (goto _label))

(event `SetHealth`
  (params (Text :type Text))
  (`/Game/Blueprints/HUD/WGT_HUD.SetText` (`self.Wgt_Damage_ref`) (`KismetTextLibrary.Conv_StringToText` (`KismetStringLibrary.Concat_StrStr` "Health: " (`KismetTextLibrary.Conv_TextToString` Text)))))

(event `RepairDamage`
  (bind _output_get (set `self.Health` (+ (`self.Health`) 20.0)))
  (`self.SetHealth` (`KismetTextLibrary.Conv_DoubleToText` _output_get "HalfToEven")))

(event `LightDamage`
  (bind _painel (`self.painel`))
  (bind _output (`|GetArrayItem` (`self.Buttons`) (`KismetMathLibrary.RandomInteger` 0)))
  (`PrimitiveComponent.SetMaterial` _painel 0 "/Game/Blueprints/SpecialMaterials/HeavyDamagePanel.HeavyDamagePanel")
  (`KismetSystemLibrary.Delay` 0.2)
  (`PrimitiveComponent.SetMaterial` _painel 0 "/Game/Meshes/Ship/PAINE_ASSETS.PAINE_ASSETS")
  (set `/Game/Blueprints/Button.bBlink` true _output)
  (if (not (`/Game/Blueprints/Button.bBlink` _output))
    (bind _output_get (set `self.Health` (- (`self.Health`) 20.0)))
    (`self.SetHealth` (`KismetTextLibrary.Conv_DoubleToText` _output_get "HalfToEven"))
    (`GameplayStatics.PlaySound2D` "/Game/VFX/WING_COMMANDER_SFX_V01_-_IMPACT_01.WING_COMMANDER_SFX_V01_-_IMPACT_01" 1.0 1.0 0.0 null null)
    (if (<= (`self.Health`) 40.0)
      (`GameplayStatics.PlaySound2D` "/Game/VFX/WING_COMMANDER_SFX_V01_-_VOZ_-_Engine_Fail.WING_COMMANDER_SFX_V01_-_VOZ_-_Engine_Fail" 1.0 1.0 0.0 null null))))

(event `HeavyDamage`
  (bind _painel (`self.painel`))
  (bind _output (`|GetArrayItem` (`self.Buttons`) (`KismetMathLibrary.RandomInteger` 3)))
  (bind _output_2 (`|GetArrayItem` (`self.Buttons`) (`KismetMathLibrary.RandomInteger` 3)))
  (`PrimitiveComponent.SetMaterial` _painel 0 "/Game/Blueprints/SpecialMaterials/HeavyDamagePanel.HeavyDamagePanel")
  (`KismetSystemLibrary.Delay` 0.2)
  (`PrimitiveComponent.SetMaterial` _painel 0 "/Game/Meshes/Ship/PAINE_ASSETS.PAINE_ASSETS")
  (if (not (`/Game/Blueprints/Button.bBlink` _output_2))
    (set `/Game/Blueprints/Button.bBlink` true _output_2)
    (if (not (`/Game/Blueprints/Button.bBlink` _output))
      (set `/Game/Blueprints/Button.bBlink` true _output)
      (set `self.Health` (- (`self.Health`) 40.0))
      (`GameplayStatics.PlaySound2D` "/Game/VFX/WING_COMMANDER_SFX_V01_-_IMPACT_03.WING_COMMANDER_SFX_V01_-_IMPACT_03" 1.0 1.0 0.0 null null))))

(fn `UserConstructionScript`)