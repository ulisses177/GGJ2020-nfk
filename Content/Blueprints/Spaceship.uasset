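; Spaceship actor that drives wingtip-style condensation and particle effects from the turning rates of the player's VrShip.
; On BeginPlay it caches the player VrShip and the Painel child actor.
; Each tick, combined pitch, yaw and roll speed above half TurnSpeed activates both particle systems and scales left and right condensation along a clamped fifth-power curve.
; Pitch enters the sum signed, unlike yaw and roll.
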(event `self.ReceiveBeginPlay`
  (bind _asvr_ship (cast `/Game/VirtualRealityBP/Blueprints/VrController/VrShip` (`GameplayStatics.GetPlayerCharacter` 0)))
  (set `self.ShipOwner` _asvr_ship)
  (bind _aspainel (cast `/Game/Blueprints/Painel` (`ChildActorComponent.ChildActor` (`self.Painel1`))))
  (set `self.Painel` _aspainel))

(event `self.ReceiveTick`
  (params (DeltaSeconds :type "Float (single-precision)"))
  (bind _lcondensation (`self.LCondensation`))
  (bind _shipowner (`self.ShipOwner`))
  (bind _turn_speed (`/Game/VirtualRealityBP/Blueprints/VrController/VrShip.Turn speed` _shipowner))
  (bind _returnvalue (+ (`/Game/VirtualRealityBP/Blueprints/VrController/VrShip.Current pitch speed` _shipowner) (`KismetMathLibrary.Abs` (`/Game/VirtualRealityBP/Blueprints/VrController/VrShip.Current yaw speed` _shipowner)) (`KismetMathLibrary.Abs` (`/Game/VirtualRealityBP/Blueprints/VrController/VrShip.Current roll speed` _shipowner))))
  (bind _returnvalue_2 (> _returnvalue (/ _turn_speed 2.0)))
  (`|ExecutionSequence`
    (:`then_0`
      (`/Engine/EditorBlueprintResources/StandardMacros.IsValid` _shipowner
        (:`Is Valid`
          (set `self.ParticlesOn` _returnvalue_2)
          (if (and _returnvalue_2 true)
            (`SceneComponent.SetRelativeScale3D` _lcondensation (* (1.85 5.0 1.0) (`KismetMathLibrary.FClamp` (`KismetMathLibrary.Abs` (/ (`KismetMathLibrary.MultiplyMultiply_FloatFloat` (* (/ _returnvalue (* _turn_speed 1.0)) 90.0) 5.0) (`KismetMathLibrary.MultiplyMultiply_FloatFloat` 80.0 5.0))))))
            (`SceneComponent.SetRelativeScale3D` (`self.RCondensation`) (* (1.85 5.0 1.0) (`KismetMathLibrary.FClamp` (`KismetMathLibrary.Abs` (/ (`KismetMathLibrary.MultiplyMultiply_FloatFloat` (* (/ _returnvalue (* _turn_speed 1.0)) 90.0) 5.0) (`KismetMathLibrary.MultiplyMultiply_FloatFloat` 80.0 5.0))))))
            (else
              (`SceneComponent.SetRelativeScale3D` _lcondensation (0.0 0.0 0.0))
              (`SceneComponent.SetRelativeScale3D` (`self.RCondensation`) (0.0 0.0 0.0)))))))
    (:`then_1`
      (`self.ToggleParticle` (`self.ParticlesOn`)))))

(event `ToggleParticle`
  (params (Condition :type Boolean))
  (`ActorComponent.SetActive` (`self.ParticleSystemL`) Condition false)
  (`ActorComponent.SetActive` (`self.ParticleSystemR`) Condition false))

(fn `UserConstructionScript`)